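; BP_Mover is an actor that moves and rotates itself from its starting transform toward a fixed offset.
; BeginPlay caches the start location and rotation.
; Tick calls Play on a timeline every frame, and its alpha drives lerps to a point offset along world X and to a half-turn rotation combined with the start rotation.
; Each timeline update applies both results together.
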(event `self.ReceiveBeginPlay`
  (set `self.startLocation` (`self.K2_GetActorLocation`))
  (set `self.startRotation` (`self.K2_GetActorRotation`)))

(event `self.ReceiveTick`
  (params (DeltaSeconds :type "Float (single-precision)"))
  (bind _startlocation (`self.startLocation`))
  (bind _startrotation (`self.startRotation`))
  (bind (_direction _lerp_move_alpha) (`Timeline|Timeline_0` :`NewTime` DeltaSeconds)
    (:`Update`
      (`self.K2_SetActorLocationAndRotation` (`KismetMathLibrary.VLerp` _startlocation (+ _startlocation (400.0 0.0 0.0)) _lerp_move_alpha) (`KismetMathLibrary.RLerp` _startrotation (`KismetMathLibrary.ComposeRotators` _startrotation (struct :`Roll` 180.0)) _lerp_move_alpha)))))

(fn `UserConstructionScript`)